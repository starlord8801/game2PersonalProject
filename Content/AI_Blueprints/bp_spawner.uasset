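; Trigger-volume spawner that creates an Ai_companion pawn the first time the player walks into it.
; BeginPlay caches the player's BP_ThirdPersonCharacter, and the Box overlap compares the entering actor against it.
; A DoOnce limits the trigger to a single aiSpawn call, which spawns the AI at the Billboard component's world location and rotation.
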(event `self.ReceiveBeginPlay`
  (bind _asbp_third_person_character (cast `/Game/ThirdPerson/Blueprints/BP_ThirdPersonCharacter` (`GameplayStatics.GetPlayerCharacter` 0)))
  (set `self.As BP Third Person Character` _asbp_third_person_character))

(event `self.Box.OnComponentBeginOverlap`
  (params (OverlappedComponent :type "PrimitiveComponent Object Reference") (OtherActor :type "Actor Object Reference") (OtherComp :type "PrimitiveComponent Object Reference") (OtherBodyIndex :type Integer) (bFromSweep :type Boolean) (SweepResult :type "HitResult Structure (by ref)"))
  (if (== OtherActor (`self.As BP Third Person Character`))
    (`/Engine/EditorBlueprintResources/StandardMacros.DoOnce` false
      (:`Completed`
        (`self.aiSpawn`)))))

(event `aiSpawn`
  (bind _billboard (`self.Billboard`))
  (`AIBlueprintHelperLibrary.SpawnAIFromClass` "/Game/AI_Blueprints/ai_companion.ai_companion_C" null (`SceneComponent.K2_GetComponentLocation` _billboard) (`SceneComponent.K2_GetComponentRotation` _billboard) false null))

(fn `UserConstructionScript`)
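; Pressure plate button that switches a linked door (DoorToActivate) on and off as actors enter and leave its Trigger volume.
; Begin and end overlap notify the door for any overlapping actor, before any type check.
; Only actors that cast to BP_ThirdPersonCharacter or ai_controller play or reverse the Plate_animation timeline, which lerps the plate's relative Z to press and raise it.
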(event `self.trigger.OnComponentBeginOverlap`
  (params (OverlappedComponent :type "PrimitiveComponent Object Reference") (OtherActor :type "Actor Object Reference") (OtherComp :type "PrimitiveComponent Object Reference") (OtherBodyIndex :type Integer) (bFromSweep :type Boolean) (SweepResult :type "HitResult Structure (by ref)"))
  (`/Game/bp_switchDoor.switchActivated` (`self.doorToActivate`))
  (`|ExecutionSequence`
    (:`then_0`
      (cast `/Game/ThirdPerson/Blueprints/BP_ThirdPersonCharacter` OtherActor)
      (bind (_direction _newtrack_0) (`Timeline|plate_animation` :!label _label)
        (:`Update`
          (`SceneComponent.K2_SetRelativeLocation` (`self.plate`) (`KismetMathLibrary.MakeVector` 0.0 0.0 (`KismetMathLibrary.Lerp` 5.0 -5.0 _newtrack_0)) false false))))
    (:`then_1`
      (cast `/Game/AI_Blueprints/ai_controller` OtherActor)
      (goto _label))))

(event `self.trigger.OnComponentEndOverlap`
  (params (OverlappedComponent :type "PrimitiveComponent Object Reference") (OtherActor :type "Actor Object Reference") (OtherComp :type "PrimitiveComponent Object Reference") (OtherBodyIndex :type Integer))
  (`/Game/bp_switchDoor.switchDeactivated` (`self.doorToActivate`))
  (`|ExecutionSequence`
    (:`then_0`
      (cast `/Game/ThirdPerson/Blueprints/BP_ThirdPersonCharacter` OtherActor)
      (goto _label :!via `Reverse`))
    (:`then_1`
      (cast `/Game/AI_Blueprints/ai_controller` OtherActor)
      (goto _label :!via `Reverse`))))

(fn `UserConstructionScript`)
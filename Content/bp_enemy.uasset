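; Enemy actor Blueprint with a simple health and death system.
; It prints a taunt on BeginPlay, and its takedamage event prints a hurt message and subtracts the incoming amount from Health.
; A CheckIfDead function tests whether Health has reached zero or below, and the actor destroys itself when it has.
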(event `self.ReceiveBeginPlay`
  (`KismetSystemLibrary.PrintString` "hello i have been programmed to destroy you"))

(event `take damage`
  (params (byAmount :type "Float (double-precision)" :default 0.2))
  (`KismetSystemLibrary.PrintString` "ouch!")
  (set `self.health` (- (`self.health`) byAmount))
  (if (`self.checkIfDead` (`self.health`))
    (`self.K2_DestroyActor`)))

(fn `checkIfDead`
  (params (health :type "Float (double-precision)"))
  (returns (isDead :type Boolean))
  (return (<= health 0.0)))

(fn `UserConstructionScript`)
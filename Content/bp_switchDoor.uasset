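; Switch-driven door Blueprint that opens once enough pressure switches are active and closes when the count drops below the requirement.
; Activation and deactivation events adjust a running count of active switches and compare it to the needed amount.
; The result plays or reverses a timeline whose track drives the door mesh's relative Z location.
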(event `switchActivated`
  (`/Engine/EditorBlueprintResources/StandardMacros.IncrementInt` (`self.pressureSwitchesActive`)
    (:`  `
      (if (>= (`self.pressureSwitchesActive`) (`self.pressureSwitchesNeeded`))
        (bind (_direction _door_position) (`Timeline|door_activate` :!label _label)
          (:`Update`
            (`SceneComponent.K2_SetRelativeLocation` (`self.door`) (`KismetMathLibrary.MakeVector` 0.0 0.0 _door_position) false false)))
        (else
          (goto _label :!via `Reverse`))))))

(event `switchDeactivated`
  (`/Engine/EditorBlueprintResources/StandardMacros.DecrementInt` (`self.pressureSwitchesActive`)
    (:`  `
      (if (>= (`self.pressureSwitchesActive`) (`self.pressureSwitchesNeeded`))
        (goto _label)
        (else
          (goto _label :!via `Reverse`))))))

(fn `UserConstructionScript`)